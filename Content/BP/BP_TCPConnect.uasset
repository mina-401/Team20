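; BP_TCPConnect is a TCP client actor that opens a socket connection to a fixed IP address and port on BeginPlay and stores the connection ID.
; Connection and disconnection callbacks print their status to the screen.
; Each received message is read as an integer, printed, and forwarded through CallMyData.
; Send and disconnect nodes exist but are not wired to run.
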(event Custom|Disconnected
  (params (ConnectionId :type Integer))
  (Development|PrintString "Disconnected"))

(event Custom|Connected
  (params (ConnectionId :type Integer))
  (Development|PrintString "Connected"))

(event Custom|ReceivedData
  (params (ConnectionId :type Integer) (Message :type Array%20of%20Bytes))
  (bind _returnvalue (Class|TcpSocketConnection|MessageReadInt Message))
  (Development|PrintString (Utilities|String|ToString(Integer) _returnvalue))
  (Default|CallMyData _returnvalue))

(event EventBeginPlay
  (bind _connectionid (Class|TcpSocketConnection|Connect "172.16.17.11" 5555 (delegate Custom|Disconnected) (delegate Custom|Connected) (delegate Custom|ReceivedData)))
  (Variables|Default|SetConnection%20Id _connectionid))

(fn ConstructionScript)