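; BP_Planet is a solar system planet actor that orbits a center point and spins on its axis.
; Construction scales the sphere by radius and places it along X by scaled sun distance.
; BeginPlay moves the actor pivot to the center, restores PlanetRoot's position, randomizes orbital yaw, and adds a hidden BP_rendertext widget.
; While IsMove is set, Tick yaws the actor and sphere at rates inversely proportional to orbital period and day length.
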(event EventBeginPlay
  (Variables|Default|SetInitialPlanetLocation (Transformation|GetActorTransform))
  (Transformation|SetActorLocationAndRotation (Variables|Default|GetCenter) (Math|Rotator|MakeRotator 0.0 0.0 0.0))
  (Transformation|SetWorldLocationAndRotation (Variables|Default|GetPlanetRoot) (.location (Variables|Default|GetInitialPlanetLocation)) (.rotation (Variables|Default|GetInitialPlanetLocation)) false false)
  (Transformation|SetActorRotation (Math|Rotator|MakeRotator 0.0 0.0 (Math|Random|RandomFloatinRange 0.0 3.6e+02)))
  (bind _returnvalue (UserInterface|CreateWidget "/Game/BP/BP_rendertext.BP_rendertext_C" (Game|GetPlayerController 0)))
  (bind _output_get (Variables|Default|SetUserWidget _returnvalue))
  (UserInterface|Viewport|AddtoViewport _output_get 0)
  (Widget|SetVisibility _output_get "Hidden"))

(event Collision|EventActorBeginOverlap
  (params (OtherActor :type Actor%20Object%20Reference)))

(event EventTick
  (params (DeltaSeconds :type Float%20%28single-precision%29))
  (bind _sphere (Variables|Default|GetSphere))
  (if (Variables|Default|GetisMove)
    (Transformation|SetActorRotation (Math|Rotator|MakeRotator 0.0 0.0 (+ (.yaw (Transformation|GetActorRotation)) (* DeltaSeconds 1e+02 (/ 88.0 (Variables|Default|GetOrbiatalPeriod))))))
    (Transformation|SetRelativeRotation _sphere (Math|Rotator|MakeRotator 0.0 0.0 (+ (.yaw (Variables|/Script/Engine.SceneComponent|GetRelativeRotation _sphere)) (* (Utilities|Time|GetWorldDeltaSeconds) 5.0 (/ 58.0 (Variables|Default|Getlenght%20of%20day))))) false false)))

(fn ConstructionScript
  (Transformation|SetWorldScale3D (Variables|Default|GetSphere) (Math|Conversions|ToVector(Float) (/ (Variables|Default|Getradius) 1.6e+02)))
  (Transformation|SetActorLocation (Math|Vector|MakeVector (* (Variables|Default|GetsunDist) (Variables|Default|Getdistance%20factor)) 0.0 0.0) false false))